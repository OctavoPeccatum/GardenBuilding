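; BP_Transmitter is a building that draws resource from a nearby BP_Source and tallies it.
; On BeginPlay it targets the closest source overlapping its owning BP_LevelStreamer's box, within the stored Distance.
; A one-second looping timer decreases the target's resource and adds a point with updated text, stopping when DecreaseResource returns true.
; Showing the building's info hides the target's arrow until the info closes.
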(event `self.ReceiveBeginPlay`
  (`parent.ReceiveBeginPlay`)
  (`self.SetTarget`)
  (bind _returnvalue (`KismetSystemLibrary.K2_SetTimer` self "GetPoint" 1.0 true))
  (set `self.GetPointTimerHandle` _returnvalue))

(event `/Game/Blueprints/Core/Interface/BPI_Interactable.BeginShowInfo`
  (params (Caller :type "Actor Object Reference"))
  (bind _target (`self.Target`))
  (`parent.BeginShowInfo` Caller)
  (`/Engine/EditorBlueprintResources/StandardMacros.IsValid` _target
    (:`Is Valid`
      (`/Game/Blueprints/Buildings/BP_Source.ShowArrow` _target false))))

(event `/Game/Blueprints/Core/Interface/BPI_Interactable.EndShowInfo`
  (bind _target (`self.Target`))
  (`parent.EndShowInfo`)
  (`/Engine/EditorBlueprintResources/StandardMacros.IsValid` _target
    (:`Is Valid`
      (`/Game/Blueprints/Buildings/BP_Source.ShowArrow` _target true))))

(fn `AddPoint`
  (set `self.Resource` (+ (`self.Resource`) 1.0))
  (`self.SetText`))

(fn `GetPoint`
  (bind _target (`self.Target`))
  (`/Engine/EditorBlueprintResources/StandardMacros.IsValid` _target
    (:`Is Valid`
      (bind _bsourceempty (`/Game/Blueprints/Buildings/BP_Source.DecreaseResource` _target))
      (if _bsourceempty
        (`KismetSystemLibrary.K2_ClearAndInvalidateTimerHandle` (`self.GetPointTimerHandle`))
        (else
          (`self.AddPoint`))))
    (:`Is Not Valid`
      _))
  (return))

(fn `SetTarget`
  (locals (Distance :type "Float (double-precision)" :default 1000000.0))
  (bind _asbp_level_streamer (cast `/Game/Blueprints/Level/BP_LevelStreamer` (`self.GetOwner`)))
  (for _array_element (`PrimitiveComponent.GetOverlappingActors` (`/Game/Blueprints/Level/BP_LevelStreamer.BoxCollision` _asbp_level_streamer) "/Game/Blueprints/Buildings/BP_Source.BP_Source_C")
    (bind _returnvalue (`KismetMathLibrary.Vector_Distance` (`self.K2_GetActorLocation` _array_element) (`self.K2_GetActorLocation`)))
    (if (< _returnvalue (`local.Distance`))
      (set `local.Distance` _returnvalue)
      (bind _asbp_source (cast `/Game/Blueprints/Buildings/BP_Source` _array_element))
      (set `self.Target` _asbp_source)))
  (return))

(fn `UserConstructionScript`
  (`parent.UserConstructionScript`))
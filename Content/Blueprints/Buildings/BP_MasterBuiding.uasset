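; BP_MasterBuiding is a building actor with a floating text label that displays its Resource value.
; The label text is formatted from Resource once at BeginPlay.
; BeginShowInfo shows the label and stores the Caller, and EndShowInfo hides it again.
; While shown, Tick turns the label's yaw to face the Caller, keeping its pitch and roll.
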(event `self.ReceiveBeginPlay`
  (`self.SetText`))

(event `self.ReceiveTick`
  (params (DeltaSeconds :type "Float (single-precision)"))
  (if (`self.bShowInfo`)
    (`self.RotateText`)))

(event `/Game/Blueprints/Core/Interface/BPI_Interactable.BeginShowInfo`
  (params (Caller :type "Actor Object Reference"))
  (`SceneComponent.SetVisibility` (`self.TextRender`) true false)
  (set `self.Caller` Caller)
  (set `self.bShowInfo` true))

(event `/Game/Blueprints/Core/Interface/BPI_Interactable.EndShowInfo`
  (`SceneComponent.SetVisibility` (`self.TextRender`) false false)
  (set `self.bShowInfo` false))

(fn `RotateText`
  (bind _textrender (`self.TextRender`))
  (bind (_returnvalue_roll _returnvalue_pitch) (`KismetMathLibrary.BreakRotator` (`SceneComponent.K2_GetComponentRotation` _textrender)))
  (bind (_returnvalue_roll_2 _returnvalue_pitch_2 _returnvalue_yaw) (`KismetMathLibrary.BreakRotator` (`KismetMathLibrary.MakeRotFromX` (- (`SceneComponent.K2_GetComponentLocation` _textrender) (`self.K2_GetActorLocation` (`self.Caller`))))))
  (`SceneComponent.K2_SetWorldRotation` (`self.TextRender`) (`KismetMathLibrary.MakeRotator` _returnvalue_roll _returnvalue_pitch (- _returnvalue_yaw 180.0)) false false))

(fn `SetMessage`
  (returns (Result :type Text))
  (return (`|FormatText` "Resource: {Resource}" (`self.Resource`))))

(fn `SetText`
  (`TextRenderComponent.K2_SetText` (`self.TextRender`) (`self.SetMessage`)))

(fn `UserConstructionScript`)
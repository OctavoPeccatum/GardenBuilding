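; BP_Source is a building actor that acts as a depletable resource source.
; DecreaseResource removes one unit per call, clamped to zero and the maximum, refreshes the text and returns an empty flag, which turns true only on a call made when already at zero.
; SetMessage formats the current and maximum resource as text, and ShowArrow sets the arrow's hidden-in-game state.
; The event graph holds only disabled default events, so the actor has no active logic there.
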(fn `DecreaseResource`
  (returns (bSourceEmpty :type Boolean))
  (if (!= (`self.Resource`) 0.0)
    (set `self.bSourceEmpty` false)
    (set `self.Resource` (`KismetMathLibrary.FClamp` (- (`self.Resource`) 1.0) 0.0 (`self.ResourceMax`)))
    (`self.SetText`)
    (else
      (set `self.bSourceEmpty` true)))
  (return (`self.bSourceEmpty`)))

(fn `SetMessage`
  (returns (Result :type Text))
  (return (`|FormatText` "Resource: {Resource}/{ResourceMax}" (`self.Resource`) (`self.ResourceMax`))))

(fn `ShowArrow`
  (params (bHidden :type Boolean))
  (`SceneComponent.SetHiddenInGame` (`self.Arrow`) bHidden false))

(fn `UserConstructionScript`
  (`parent.UserConstructionScript`))
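; Player controller that creates the HUD and moves the character between an indexed chain of level streamer actors, with an escape menu that pauses the game.
; Next-map input reuses the stored level or spawns a new streamer at the previous one's attach point; previous-map only revisits stored levels.
; Each switch teleports the character, toggles actor visibility and updates its current level behind a briefly shown loading screen.
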(event `self.ReceiveBeginPlay`
  (bind _returnvalue (`|CreateWidget` "/Game/Blueprints/Core/UI/WBP_PlayerHUD.WBP_PlayerHUD_C" self))
  (`UserWidget.AddToViewport` _returnvalue 0))

(event `self.ReceivePossess`
  (params (PossessedPawn :type "Pawn Object Reference"))
  (bind _asbp_character (cast `/Game/Blueprints/Core/Pawn/PlayerCharacter/BP_Character` PossessedPawn))
  (set `self.As BP Character` _asbp_character)
  (bind _returnvalue (`GameplayStatics.GetActorOfClass` "/Game/Blueprints/Level/BP_LevelStreamer.BP_LevelStreamer_C"))
  (`BlueprintMapLibrary.Map_Add` (`self.Levels`) (`self.Iterator`) _returnvalue)
  (`self.UpdateCharacterLevel`))

(event `InputAction|NextMap`
  (params (Key :type "Key Structure"))
  (:`Pressed`
    (bind _returnvalue (`|CreateWidget` "/Game/Blueprints/Core/UI/WBP_LoadingScreen.WBP_LoadingScreen_C" self))
    (`UserWidget.AddToViewport` _returnvalue 0)
    (bind _result (`/Engine/EditorBlueprintResources/StandardMacros.IncrementInt` (`self.Iterator`))
      (:`  `
        (bind (_value _returnvalue_2) (`BlueprintMapLibrary.Map_Find` (`self.Levels`) _result))
        (if _returnvalue_2
          (`self.TeleportCharacter` _value)
          (`/Game/Blueprints/Level/BP_LevelStreamer.HideAllActors` _value false)
          (else
            (bind _returnvalue_3 (`|SpawnActorFromClass` "/Game/Blueprints/Level/BP_LevelStreamer.BP_LevelStreamer_C" (`KismetMathLibrary.MakeTransform` (`SceneComponent.K2_GetComponentLocation` (`/Game/Blueprints/Level/BP_LevelStreamer.PointToNewLevel` (`BlueprintMapLibrary.Map_Find` (`self.Levels`) (- (`self.Iterator`) 1))))) "Undefined" "OverrideRootScale" null null))
            (`BlueprintMapLibrary.Map_Add` (`self.Levels`) (`self.Iterator`) _returnvalue_3)
            (`self.TeleportCharacter` _returnvalue_3)))
        (`/Game/Blueprints/Level/BP_LevelStreamer.HideAllActors` (`BlueprintMapLibrary.Map_Find` (`self.Levels`) (- (`self.Iterator`) 1)) true)
        (`self.UpdateCharacterLevel`)
        (`KismetSystemLibrary.Delay` 0.5)
        (`Widget.RemoveFromParent` _returnvalue)))))

(event `InputAction|PreviousMap`
  (params (Key :type "Key Structure"))
  (:`Pressed`
    (bind _result (`/Engine/EditorBlueprintResources/StandardMacros.DecrementInt` (`self.Iterator`))
      (:`  `
        (bind (_value _returnvalue) (`BlueprintMapLibrary.Map_Find` (`self.Levels`) _result))
        (if _returnvalue
          (bind _returnvalue_2 (`|CreateWidget` "/Game/Blueprints/Core/UI/WBP_LoadingScreen.WBP_LoadingScreen_C" self))
          (`UserWidget.AddToViewport` _returnvalue_2 0)
          (`self.TeleportCharacter` _value)
          (`/Game/Blueprints/Level/BP_LevelStreamer.HideAllActors` _value false)
          (`/Game/Blueprints/Level/BP_LevelStreamer.HideAllActors` (`BlueprintMapLibrary.Map_Find` (`self.Levels`) (+ (`self.Iterator`) 1)) true)
          (`self.UpdateCharacterLevel`)
          (`KismetSystemLibrary.Delay` 0.5)
          (`Widget.RemoveFromParent` _returnvalue_2)
          (else
            (`/Engine/EditorBlueprintResources/StandardMacros.IncrementInt` (`self.Iterator`))))))))

(event `InputAction|EscapeMenu`
  (params (Key :type "Key Structure"))
  (:`Pressed`
    (`self.DisableInput` self)
    (`WidgetBlueprintLibrary.SetInputMode_UIOnlyEx` self null)
    (set `self.bShowMouseCursor` true)
    (bind _returnvalue (`|CreateWidget` "/Game/Blueprints/Core/UI/WBP_EscapeMenu.WBP_EscapeMenu_C" self))
    (`UserWidget.AddToViewport` _returnvalue 0)
    (set `self.EscapeMenu` _returnvalue)
    (`GameplayStatics.SetGamePaused` true)))

(fn `ExitGame`
  (`KismetSystemLibrary.QuitGame` self "Quit"))

(fn `Resume`
  (`self.EnableInput` self)
  (`WidgetBlueprintLibrary.SetInputMode_GameOnly` self)
  (set `self.bShowMouseCursor` false)
  (`Widget.RemoveFromParent` (`self.EscapeMenu`))
  (`GameplayStatics.SetGamePaused` false))

(fn `TeleportCharacter`
  (params (Level :type "/Game/Blueprints/Level/BP_LevelStreamer Object Reference"))
  (`self.K2_SetActorLocation` (`self.As BP Character`) (`SceneComponent.K2_GetComponentLocation` (`/Game/Blueprints/Level/BP_LevelStreamer.Capsule` Level)) false false)
  (return))

(fn `UpdateCharacterLevel`
  (`/Game/Blueprints/Core/Pawn/PlayerCharacter/BP_Character.SetCurrentLevel` (`self.As BP Character`) (`BlueprintMapLibrary.Map_Find` (`self.Levels`) (`self.Iterator`))))

(fn `UserConstructionScript`)